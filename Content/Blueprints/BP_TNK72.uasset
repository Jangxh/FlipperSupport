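; BP_TNK72 is a player-driven tank pawn that feeds Enhanced Input into its vehicle movement component and controller-based camera look with clamped pitch.
; Two control schemes coexist: direct throttle, brake/reverse and turn actions, plus left/right track inputs that CalcTankThrottleAndSteering averages into throttle and subtracts into yaw.
; Turn input eases toward its starting value, and Tick sets a flag that zeroes it when mesh angular speed exceeds a threshold.
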(event Input|EnhancedActionEvents|EnhancedInputActionIA_MoveForward
  (params (ActionValue :type Float%20%28double-precision%29) (ElapsedSeconds :type Float%20%28double-precision%29) (TriggeredSeconds :type Float%20%28double-precision%29) (InputAction :type Input%20Action%20Object%20Reference :default "/Game/Blueprints/Input/Actions/IA_MoveForward.IA_MoveForward"))
  (:Triggered
    (Class|ChaosVehicleMovementComponent|SetThrottleInput (Variables|Default|GetVehicleMovementComponent) ActionValue :!label _label))
  (:Completed
    (goto _label)))

(event Input|EnhancedActionEvents|EnhancedInputActionIA_LookAround
  (params (ActionValue :type Vector%202D%20Structure) (ElapsedSeconds :type Float%20%28double-precision%29) (TriggeredSeconds :type Float%20%28double-precision%29) (InputAction :type Input%20Action%20Object%20Reference :default "/Game/Blueprints/Input/Actions/IA_LookAround.IA_LookAround"))
  (Pawn|Input|AddControllerYawInput (.x ActionValue))
  (Pawn|Input|AddControllerPitchInput (.y ActionValue)))

(event Input|EnhancedActionEvents|EnhancedInputActionIA_Turn
  (params (ActionValue :type Float%20%28double-precision%29) (ElapsedSeconds :type Float%20%28double-precision%29) (TriggeredSeconds :type Float%20%28double-precision%29) (InputAction :type Input%20Action%20Object%20Reference :default "/Game/Blueprints/Input/Actions/IA_Turn.IA_Turn"))
  (:Triggered
    (if (Variables|Default|GetbStopTurn)
      (Class|ChaosVehicleMovementComponent|SetYawInput (Variables|Default|GetVehicleMovementComponent) 0.0)
      (else
        (bind _output_get (Variables|Default|SetCurrentYawInput (Math|Float|Lerp (Variables|Default|GetCurrentYawInput) (Variables|Default|GetTargetYawInput) 0.15)))
        (Class|ChaosVehicleMovementComponent|SetYawInput (Variables|Default|GetVehicleMovementComponent) _output_get))))
  (:Started
    (Variables|Default|SetTargetYawInput ActionValue)
    (Variables|Default|SetCurrentYawInput 0.0))
  (:Completed
    (Class|ChaosVehicleMovementComponent|SetYawInput (Variables|Default|GetVehicleMovementComponent) ActionValue)))

(event Input|EnhancedActionEvents|EnhancedInputActionIA_LeftMoveForward
  (params (ActionValue :type Float%20%28double-precision%29) (ElapsedSeconds :type Float%20%28double-precision%29) (TriggeredSeconds :type Float%20%28double-precision%29) (InputAction :type Input%20Action%20Object%20Reference :default "/Game/Blueprints/Input/Actions/IA_LeftMoveForward.IA_LeftMoveForward"))
  (:Triggered
    (Variables|Default|SetLeftThrottleInput ActionValue :!label _label)
    (CallFunction|CalcTankThrottleandSteering))
  (:Completed
    (goto _label)))

(event Input|EnhancedActionEvents|EnhancedInputActionIA_TankBrake
  (params (ActionValue :type Float%20%28double-precision%29) (ElapsedSeconds :type Float%20%28double-precision%29) (TriggeredSeconds :type Float%20%28double-precision%29) (InputAction :type Input%20Action%20Object%20Reference :default "/Game/Blueprints/Input/Actions/IA_TankBrake.IA_TankBrake"))
  (:Triggered
    (Class|ChaosVehicleMovementComponent|SetBrakeInput (Variables|Default|GetVehicleMovementComponent) ActionValue :!label _label))
  (:Completed
    (goto _label)))

(event Input|EnhancedActionEvents|EnhancedInputActionIA_Reverse
  (params (ActionValue :type Float%20%28double-precision%29) (ElapsedSeconds :type Float%20%28double-precision%29) (TriggeredSeconds :type Float%20%28double-precision%29) (InputAction :type Input%20Action%20Object%20Reference :default "/Game/Blueprints/Input/Actions/IA_Reverse.IA_Reverse"))
  (:Triggered
    (Class|ChaosVehicleMovementComponent|SetBrakeInput (Variables|Default|GetVehicleMovementComponent) ActionValue :!label _label))
  (:Completed
    (goto _label)))

(event Input|EnhancedActionEvents|EnhancedInputActionIA_RightMoveForward
  (params (ActionValue :type Float%20%28double-precision%29) (ElapsedSeconds :type Float%20%28double-precision%29) (TriggeredSeconds :type Float%20%28double-precision%29) (InputAction :type Input%20Action%20Object%20Reference :default "/Game/Blueprints/Input/Actions/IA_RightMoveForward.IA_RightMoveForward"))
  (:Triggered
    (Variables|Default|SetRightThrottleInput ActionValue :!label _label)
    (CallFunction|CalcTankThrottleandSteering))
  (:Completed
    (goto _label)))

(event EventBeginPlay
  (bind _returnvalue (Game|GetPlayerController 0))
  (bind _returnvalue_2 (Game|GetPlayerCameraManager 0))
  (bind _returnvalue_3 (PlayerController|LocalPlayerSubsystems|GetEnhancedInputLocalPlayerSubsystem _returnvalue))
  (Utilities|IsValid _returnvalue_3
    (:Is%20Valid
      (Input|AddMappingContext _returnvalue_3 "/Game/Blueprints/Input/IMC_Tank.IMC_Tank" 0 "(bIgnoreAllPressedKeysUntilRelease=True,bForceImmediately=False,bNotifyUserSettings=False)")
      (Variables|/Script/Engine.PlayerCameraManager|SetViewPitchMin _returnvalue_2 -6e+01)
      (Variables|/Script/Engine.PlayerCameraManager|SetViewPitchMax _returnvalue_2 15.0))))

(event EventTick
  (params (DeltaSeconds :type Float%20%28single-precision%29))
  (Variables|Default|SetbStopTurn (> (Math|Vector|VectorLength (Physics|GetPhysicsAngularVelocityinDegrees (Variables|Character|GetMesh) "None")) 72.0)))

(fn ConstructionScript)

(fn CalcTankThrottleandSteering
  (Class|ChaosVehicleMovementComponent|SetThrottleInput (Variables|Default|GetVehicleMovementComponent) (/ (+ (Variables|Default|GetLeftThrottleInput) (Variables|Default|GetRightThrottleInput)) 2.0))
  (Class|ChaosVehicleMovementComponent|SetYawInput (Variables|Default|GetVehicleMovementComponent) (- (Variables|Default|GetRightThrottleInput) (Variables|Default|GetLeftThrottleInput))))