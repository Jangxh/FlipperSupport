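; Player-controlled tank Blueprint (TNK72) driven by separate left and right throttle inputs.
; On BeginPlay it adds the IMC_Tank Enhanced Input context and clamps camera pitch; look input rotates the controller.
; Each side's triggered and completed input events feed the matching vehicle movement throttle.
; Key 1 applies a huge force to the mesh root bone, passing the world forward vector as a local-space force.
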(event Input|EnhancedActionEvents|EnhancedInputActionIA_LookAround
  (params (ActionValue :type Vector%202D%20Structure) (ElapsedSeconds :type Float%20%28double-precision%29) (TriggeredSeconds :type Float%20%28double-precision%29) (InputAction :type Input%20Action%20Object%20Reference :default "/Game/Blueprints/Input/Actions/IA_LookAround.IA_LookAround"))
  (Pawn|Input|AddControllerYawInput (.x ActionValue))
  (Pawn|Input|AddControllerPitchInput (.y ActionValue)))

(event Input|EnhancedActionEvents|EnhancedInputActionIA_LeftMoveForward
  (params (ActionValue :type Float%20%28double-precision%29) (ElapsedSeconds :type Float%20%28double-precision%29) (TriggeredSeconds :type Float%20%28double-precision%29) (InputAction :type Input%20Action%20Object%20Reference :default "/Game/Blueprints/Input/Actions/IA_LeftMoveForward.IA_LeftMoveForward"))
  (:Triggered
    (Class|CTankMovementComponent|SetLeftThrottle (Variables|Default|GetVehicleMovementComponent) ActionValue :!label _label))
  (:Completed
    (goto _label)))

(event Input|EnhancedActionEvents|EnhancedInputActionIA_RightMoveForward
  (params (ActionValue :type Float%20%28double-precision%29) (ElapsedSeconds :type Float%20%28double-precision%29) (TriggeredSeconds :type Float%20%28double-precision%29) (InputAction :type Input%20Action%20Object%20Reference :default "/Game/Blueprints/Input/Actions/IA_RightMoveForward.IA_RightMoveForward"))
  (:Triggered
    (Class|CTankMovementComponent|SetRightThrottle (Variables|Default|GetVehicleMovementComponent) ActionValue :!label _label))
  (:Completed
    (goto _label)))

(event EventBeginPlay
  (bind _returnvalue (Game|GetPlayerController 0))
  (bind _returnvalue_2 (Game|GetPlayerCameraManager 0))
  (bind _returnvalue_3 (PlayerController|LocalPlayerSubsystems|GetEnhancedInputLocalPlayerSubsystem _returnvalue))
  (Utilities|IsValid _returnvalue_3
    (:Is%20Valid
      (Input|AddMappingContext _returnvalue_3 "/Game/Blueprints/Input/IMC_Tank.IMC_Tank" 0 "(bIgnoreAllPressedKeysUntilRelease=True,bForceImmediately=False,bNotifyUserSettings=False)")
      (Variables|/Script/Engine.PlayerCameraManager|SetViewPitchMin _returnvalue_2 -6e+01)
      (Variables|/Script/Engine.PlayerCameraManager|SetViewPitchMax _returnvalue_2 15.0))))

(event Input|KeyboardEvents|1
  (params (Key :type Key%20Structure :default "None"))
  (:Pressed
    (Class|PrimitiveComponent|AddForceatLocationLocal (Variables|Character|GetMesh) (* (Transformation|GetActorForwardVector) 1e+09) "0, 0, 0" "root")))

(fn ConstructionScript)